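; BP_Sevens drives the player-facing UI for a Sevens card game, from in-play counters to the result screen.
; On BeginPlay it creates the default HUD widget, then pushes the player's card and pass counts into it every Tick.
; Tick also polls the EndGame flag, clearing it on first detection, setting EndGameValue and showing the result widget with the player's ranking.
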(event EventBeginPlay
  (bind _returnvalue (UserInterface|CreateWidget "/Game/shuby/UIs/WB_DefaultUI.WB_DefaultUI_C"))
  (UserInterface|Viewport|AddtoViewport _returnvalue 0))

(event EventTick
  (params (DeltaSeconds :type Float%20%28single-precision%29))
  (Default|SetCardNum (stale EventBeginPlay _returnvalue) (Variables|Default|GetPlayerCardNum))
  (Default|SetPassNum (stale EventBeginPlay _returnvalue) (Variables|Default|GetPlayerPassNum))
  (if (Variables|Default|GetendGame)
    (Variables|Default|SetendGame false)
    (Variables|Default|SetEndGameValue true)
    (bind _returnvalue (UserInterface|CreateWidget "/Game/shuby/UIs/WB_SevensResult.WB_SevensResult_C"))
    (UserInterface|Viewport|AddtoViewport _returnvalue 0)
    (Default|SetRankText _returnvalue (Utilities|String|ToString(Integer) (Variables|Default|GetRanking)))))

(fn ConstructionScript)